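; BP_Enemy is an enemy that chases the player's BP_Kart.
; On BeginPlay it casts the player pawn to BP_Kart, caches it and issues AIMoveTo with the kart as target actor, reissuing the move only on success.
; Tick stores the kart's location in PlayerPOS, which is also passed as the move destination.
; A debug string prints on each move attempt.
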(event Custom|Move%20Towrds%20Player
  (Development|PrintString "Enemy move :)")
  (bind _asbp_kart (Utilities|Casting|CastToBP_Kart (Game|Player|GetPlayerPawn 0)))
  (bind _output_get (Variables|Default|SetBP%20Kart _asbp_kart))
  (AI|AIMoveTo self (Variables|Default|GetPlayer%20POS) _output_get 5.0 false
    (:OnSuccess
      (CallFunction|MoveTowrdsPlayer))))

(event Custom|Get%20Player%20Position
  (Variables|Default|SetPlayer%20POS (Transformation|GetActorLocation (Variables|Default|GetBP%20Kart))))

(event EventTick
  (params (DeltaSeconds :type Float%20%28single-precision%29))
  (CallFunction|GetPlayerPosition))

(event EventBeginPlay
  (CallFunction|MoveTowrdsPlayer))

(fn ConstructionScript)