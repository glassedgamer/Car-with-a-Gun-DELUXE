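; Player-driven physics kart that shoots limited-ammo bullets and loses health when it overlaps enemies, destroying them.
; Each tick, four wheel line traces apply compression-scaled suspension forces to the body and reposition wheel children.
; Each wheel also applies forward thrust, even airborne, from an interpolated, decaying throttle that shifts center of mass and spins wheels.
; Enhanced Input drives throttle, torque-based steering and firing; BeginPlay adds HUD and tutorial widgets.
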(event Input|EnhancedActionEvents|EnhancedInputActionIA_Accelerate
  (params (ActionValue :type Float%20%28double-precision%29) (ElapsedSeconds :type Float%20%28double-precision%29) (TriggeredSeconds :type Float%20%28double-precision%29) (InputAction :type Input%20Action%20Object%20Reference :default "/Game/Player/Inputs/IA_Accelerate.IA_Accelerate"))
  ;[0.15 0.15 0.15 0.5] Player Inputs
  ;;[0.15 0.15 0.15 0.5] Accelerate
  (Variables|Default|SetAccelerationInput (Math|Interpolation|FInterpTo (Variables|Default|GetAccelerationInput) ActionValue (Utilities|Time|GetWorldDeltaSeconds) 0.5)))

(event Input|EnhancedActionEvents|EnhancedInputActionIA_Steer
  (params (ActionValue :type Float%20%28double-precision%29) (ElapsedSeconds :type Float%20%28double-precision%29) (TriggeredSeconds :type Float%20%28double-precision%29) (InputAction :type Input%20Action%20Object%20Reference :default "/Game/Player/Inputs/IA_Steer.IA_Steer"))
  ;[0.15 0.15 0.15 0.5] Player Inputs
  ;;[0.15 0.15 0.15 0.5] Steering
  (Class|PrimitiveComponent|AddTorqueinRadians (Variables|Default|GetBox) (Math|Vector|MakeVector 0.0 0.0 (* ActionValue 1e+06 (Variables|Default|GetAccelerationInput))) "None" false)
  (CallFunction|TurnWheels ActionValue))

(event Input|EnhancedActionEvents|EnhancedInputActionIA_PewPew
  (params (ActionValue :type Boolean) (ElapsedSeconds :type Float%20%28double-precision%29) (TriggeredSeconds :type Float%20%28double-precision%29) (InputAction :type Input%20Action%20Object%20Reference :default "/Game/Player/Inputs/IA_PewPew.IA_PewPew"))
  ;[0.15 0.15 0.15 0.5] Player Inputs
  ;;[0.15 0.15 0.15 0.5] Shooting
  (if (> (Variables|Default|GetAmmoCount) 0)
    (Variables|Default|SetAmmoCount (- (Variables|Default|GetAmmoCount) 1))
    (Game|SpawnActorfromClass "/Game/Player/Bullet.Bullet_C" (Transformation|GetWorldTransform (Variables|Default|GetGun_Pos)) "AlwaysSpawn" "MultiplyWithRoot" 0 0)))

(event EventTick
  (params (DeltaSeconds :type Float%20%28single-precision%29))
  ;[0.15 0.15 0.15 0.5] Wheel Suspension
  (CallFunction|SuspensionCast (Variables|Default|GetFL_Wheel))
  (CallFunction|SuspensionCast (Variables|Default|GetFR_Wheel))
  (CallFunction|SuspensionCast (Variables|Default|GetBR_Wheel))
  (CallFunction|SuspensionCast (Variables|Default|GetBL_Wheel))
  (CallFunction|CalculateAcceleration))

(event EventBeginPlay
  ;[0.15 0.15 0.15 0.5] Get Input System & Mappings
  (Input|AddMappingContext (PlayerController|LocalPlayerSubsystems|GetEnhancedInputLocalPlayerSubsystem (Game|GetPlayerController 0)) "/Game/Player/Inputs/IMC_Vehicle.IMC_Vehicle" 0 "(bIgnoreAllPressedKeysUntilRelease=True,bForceImmediately=False,bNotifyUserSettings=False)")
  ;[0.15 0.15 0.15 0.5] Add HUD to screen
  (bind _returnvalue (UserInterface|CreateWidget "/Game/Player/UI/General_UI.General_UI_C"))
  (UserInterface|Viewport|AddtoViewport _returnvalue 0)
  (bind _returnvalue_2 (UserInterface|CreateWidget "/Game/UI/Tutorial.Tutorial_C"))
  (UserInterface|Viewport|AddtoViewport _returnvalue_2 0)
  (Variables|Default|SetAmmoCount 30)
  (Variables|Default|SetHealth (Variables|Default|GetMaxHealth)))

(event Collision|EventActorBeginOverlap
  (params (OtherActor :type Actor%20Object%20Reference))
  ;[0.15 0.15 0.15 0.5] Enemy collisions
  (bind _asbp_enemy (Utilities|Casting|CastToBP_Enemy OtherActor))
  (Actor|DestroyActor _asbp_enemy)
  (Variables|Default|SetHealth (- (Variables|Default|GetHealth) 1e+01)))

(fn ConstructionScript)

(fn SuspensionCast
  (params (Wheel%20Comp :type Scene%20Component%20Object%20Reference))
  (bind _returnvalue (Transformation|GetWorldLocation Wheel%20Comp))
  (bind _returnvalue_2 (Components|GetChildComponent Wheel%20Comp 0))
  (bind _outhit (Collision|LineTraceByChannel _returnvalue (+ _returnvalue (* (Math|Vector|GetUpVector Wheel%20Comp) -6e+01)) "TraceTypeQuery1" false 0 "ForOneFrame")) ; UE5 Raycast method
  (if (.bBlockingHit (Collision|BreakHitResult _outhit))
    (Class|PrimitiveComponent|AddForceatLocation (Variables|Default|GetBox) (* (- 1.0 (Math|Float|NormalizetoRange (.Distance (Collision|BreakHitResult _outhit)) 0.0 6e+01)) (Math|Vector|GetUnitDirection(Vector) (.TraceEnd (Collision|BreakHitResult _outhit)) (.TraceStart (Collision|BreakHitResult _outhit))) 1e+05) (Transformation|GetWorldLocation Wheel%20Comp) "None")
    (CallFunction|AccelerateKart Wheel%20Comp)
    (Transformation|SetRelativeLocation _returnvalue_2 (Math|Vector|MakeVector 0.0 0.0 (Math|Interpolation|FInterpTo (.z (Variables|/Script/Engine.SceneComponent|GetRelativeLocation _returnvalue_2)) (+ (* (.Distance (Collision|BreakHitResult _outhit)) -1.0) 32.0) (Utilities|Time|GetWorldDeltaSeconds) 3.0)) false false)
    (else
      (CallFunction|AccelerateKart Wheel%20Comp))))

(fn CalculateAcceleration
  (bind _output_get (Variables|Default|SetAcceleration (* (Math|Float|Lerp 0.0 1.5e+04 (Variables|Default|GetAccelerationInput)) (Variables|Default|GetAccelerationInput))))
  (Variables|Default|SetAccelerationInput (Math|Interpolation|FInterpTo (Variables|Default|GetAccelerationInput) 0.0 (Utilities|Time|GetWorldDeltaSeconds) 0.3))
  (Transformation|AddLocalRotation (Variables|Default|GetWheel_BL) (Math|Rotator|MakeRotator 0.0 (/ _output_get -1e+03) 0.0) false false))

(fn AccelerateKart
  (params (Target :type Scene%20Component%20Object%20Reference))
  (bind _box (Variables|Default|GetBox))
  (Class|PrimitiveComponent|AddForceatLocation (Variables|Default|GetBox) (* (Math|Vector|GetForwardVector _box) (Variables|Default|GetSpeedForce) (Variables|Default|GetAccelerationInput) (Physics|GetMass _box)) (Transformation|GetWorldLocation Target) "None")
  (Class|PrimitiveComponent|SetCenterOfMass (Variables|Default|GetBox) (* "50.000000,0.000000,0.000000" (Variables|Default|GetAccelerationInput)) "None"))

(fn AddAmmo
  (Variables|Default|SetAmmoCount (+ (Variables|Default|GetAmmoCount) 5))
  (if (> (Variables|Default|GetAmmoCount) (Variables|Default|GetMaxAmmo))
    (Variables|Default|SetAmmoCount (Variables|Default|GetMaxAmmo))))

(fn TurnWheels
  (params (Target :type Float%20%28double-precision%29))
  (Transformation|SetRelativeRotation (Variables|Default|GetFL_Wheel) (Math|Rotator|MakeRotator 0.0 0.0 (Math|Interpolation|FInterpTo (.yaw (Variables|/Script/Engine.SceneComponent|GetRelativeRotation (Variables|Default|GetFR_Wheel))) Target (Utilities|Time|GetWorldDeltaSeconds) 3.0)) false false))